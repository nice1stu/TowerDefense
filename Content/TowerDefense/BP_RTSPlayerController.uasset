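; RTS player controller for the tower defense game that drives marquee selection from the left mouse button.
; On BeginPlay it sets Game and UI input with the mouse always locked to the viewport and hides the system cursor.
; It forwards press and release to the HUD as messages, and uses a pressed flag to send a held message every Tick during a drag.
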(event EventBeginPlay
  (Input|SetInputModeGameandUI self 0 "LockAlways" true false)
  (Variables|Default|SetbShowMouseCursor false))

(event EventTick
  (params (DeltaSeconds :type Float%20%28single-precision%29))
  (if (Variables|Default|GetIsLMBPressed)
    (Class|BPIRTSInterface|MarqueeHeld(Message) (HUD|GetHUD))))

(event Input|MouseEvents|LeftMouseButton
  (params (Key :type Key%20Structure :default "None"))
  (bind _returnvalue (HUD|GetHUD))
  (:Pressed
    (Variables|Default|SetIsLMBPressed true)
    (Class|BPIRTSInterface|MarqueePressed(Message) _returnvalue))
  (:Released
    (Variables|Default|SetIsLMBPressed false)
    (Class|BPIRTSInterface|MarqueeReleased(Message) _returnvalue)))

(fn ConstructionScript)