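; HUD that provides RTS-style drag-box unit selection in a tower defense game.
; Marquee pressed, held and released events track the mouse corners and toggle drawing.
; While active, DrawHUD renders a translucent green rectangle and queries all actors inside it every frame.
; It sends select messages to enclosed actors and release messages to those that leave, keeping SelectedUnits in sync until the drag ends.
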(event EventMarqueePressed
  (bind _returnvalue (Game|GetPlayerController 0))
  (bind (_locationx _locationy) (Game|Player|GetMousePosition _returnvalue))
  (Variables|Default|SetIsDrawing true)
  (bind _output_get (Variables|Default|SetMouseStartPosition (Math|Vector2D|MakeVector2D _locationx _locationy)))
  (Variables|Default|SetMouseCurrentPosition (Math|Vector2D|MakeVector2D (.x _output_get) (.y _output_get))))

(event EventMarqueeHeld
  (bind _returnvalue (Game|GetPlayerController 0))
  (bind (_locationx _locationy) (Game|Player|GetMousePosition _returnvalue))
  (Variables|Default|SetMouseCurrentPosition (Math|Vector2D|MakeVector2D _locationx _locationy)))

(event EventMarqueeReleased
  (Variables|Default|SetIsDrawing false))

(event EventDrawHUD
  (params (SizeX :type Integer) (SizeY :type Integer))
  (bind _mousestartposition (Variables|Default|GetMouseStartPosition))
  (bind _mousecurrentposition (Variables|Default|GetMouseCurrentPosition))
  (if (Variables|Default|GetIsDrawing)
    (HUD|DrawRect "(R=0.000000,G=1.000000,B=0.000000,A=0.200000)" (.x _mousestartposition) (.y _mousestartposition) (- (.x _mousecurrentposition) (.x _mousestartposition)) (- (.y _mousecurrentposition) (.y _mousestartposition)))
    (bind _output_get (Variables|Default|SetActorsInSelection (Class|HUD|GetActorsinSelectionRectangle "/Script/Engine.Actor" (Variables|Default|GetMouseStartPosition) (Variables|Default|GetMouseCurrentPosition) false false)))
    (for _array_element _output_get
      (Class|BPIRTSInterface|SelectUnit(Message) _array_element)
      (Utilities|Array|AddUnique (Variables|Default|GetSelectedUnits) _array_element))
    (for _array_element_2 (Variables|Default|GetSelectedUnits)
      (if (== (Utilities|Array|FindItem (Variables|Default|GetActorsInSelection) _array_element_2) -1)
        (Class|BPIRTSInterface|ReleaseUnit(Message) _array_element_2)
        (Utilities|Array|RemoveItem (Variables|Default|GetSelectedUnits) _array_element_2)))))

(fn ConstructionScript)