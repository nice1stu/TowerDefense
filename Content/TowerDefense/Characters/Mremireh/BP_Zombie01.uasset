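; BP_Zombie01 is a tower defense zombie enemy that heads for the player's base once it sees a pawn.
; Pawn sensing sets SeePlayer and triggers GotoPlayer, which issues an AI move toward each actor tagged PlayerBase.
; A successful move calls Attack, which is a placeholder that only prints a message.
; An unconnected cast to the ABP_Mremireh animation Blueprint would set IsAttacking but never runs.
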(event OnSeePawn(PawnSensing)
  (params (Pawn :type Pawn%20Object%20Reference))
  (Variables|Default|SetSeePlayer true)
  (CallFunction|GotoPlayer))

(event Custom|Attack
  (Development|PrintString "ATTACK !" true true "(R=1.000000,G=0.000000,B=0.000000,A=1.000000)"))

(event Custom|Goto%20Player
  (if (Variables|Default|GetSeePlayer)
    (bind _outactors (Actor|GetAllActorswithTag "PlayerBase"))
    (for _array_element _outactors
      (AI|AIMoveTo self "0, 0, 0" _array_element 1e+01 false
        (:OnSuccess
          (CallFunction|Attack))))))

(event EventBeginPlay
  (|CallParentFunction) ; This node is disabled and will not be called.\nDrag off pins to build functionality.
)

(event Collision|EventActorBeginOverlap
  (params (OtherActor :type Actor%20Object%20Reference))
  (|CallParentFunction OtherActor) ; This node is disabled and will not be called.\nDrag off pins to build functionality.
)

(event EventTick
  (params (DeltaSeconds :type Float%20%28single-precision%29))
  (|CallParentFunction DeltaSeconds) ; This node is disabled and will not be called.\nDrag off pins to build functionality.
)

(fn ConstructionScript
  (|CallParentFunction))