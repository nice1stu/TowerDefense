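; RTS-style camera pawn for the tower defense game, with axis-driven panning, yaw rotation and spring-arm zoom.
; Forward and right inputs add movement along the actor's own axes, so panning follows the yaw set by the rotate input.
; Zoom input adjusts a clamped target arm length, which the spring arm smoothly interpolates toward from its starting length of half the maximum.
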(event EventBeginPlay
  (bind _output_get (Variables|/Script/Engine.SpringArmComponent|SetTargetArmLength (Variables|Default|GetSpringArm) (* (Variables|Default|GetMaxZoomable) 0.5)))
  (Variables|Default|SetNewTargetArmLength _output_get))

(event Collision|EventActorBeginOverlap
  (params (OtherActor :type Actor%20Object%20Reference)))

(event EventTick
  (params (DeltaSeconds :type Float%20%28single-precision%29)))

(event Input|AxisEvents|InputAxisMoveForward
  (params (AxisValue :type Float%20%28single-precision%29))
  ;[1 1 1] Camera Controls
  (CallFunction|MoveForward AxisValue))

(event Input|AxisEvents|InputAxisMoveRight
  (params (AxisValue :type Float%20%28single-precision%29))
  ;[1 1 1] Camera Controls
  (CallFunction|MoveRight AxisValue))

(event Input|AxisEvents|InputAxisRotateCamera
  (params (AxisValue :type Float%20%28single-precision%29))
  ;[1 1 1] Camera Controls
  (CallFunction|RotateCamera AxisValue))

(event Input|AxisEvents|InputAxisZoomCamera
  (params (AxisValue :type Float%20%28single-precision%29))
  ;[1 1 1] Camera Controls
  (CallFunction|ZoomCamera AxisValue))

(event Input|MouseEvents|LeftMouseButton
  (params (Key :type Key%20Structure :default "None")))

(fn ConstructionScript)

(fn MoveForward
  (params (AxisValue :type Float%20%28double-precision%29))
  (Pawn|Input|AddMovementInput (Transformation|GetActorForwardVector) (* AxisValue (Variables|Default|GetCameraMoveSpeed)) false))

(fn MoveRight
  (params (AxisValue :type Float%20%28double-precision%29))
  (Pawn|Input|AddMovementInput (Transformation|GetActorRightVector) (* AxisValue (Variables|Default|GetCameraMoveSpeed)) false))

(fn RotateCamera
  (params (AxisValue :type Float%20%28double-precision%29))
  (bind _returnvalue (Transformation|GetActorRotation))
  (bind (_roll _pitch _yaw) (Math|Rotator|BreakRotator _returnvalue))
  (Transformation|SetActorRotation (Math|Rotator|MakeRotator _roll _pitch (+ (* AxisValue (Variables|Default|GetCameraRotateSpeed)) _yaw)))
  (return))

(fn ZoomCamera
  (params (AxisValue :type Float%20%28double-precision%29))
  (bind _springarm (Variables|Default|GetSpringArm))
  (bind _output_get (Variables|Default|SetNewTargetArmLength (Math|Float|Clamp(Float) (+ (* AxisValue (Variables|Default|GetZoomSpeed)) (Variables|Default|GetNewTargetArmLength)) (Variables|Default|GetMinZoomable) (Variables|Default|GetMaxZoomable))))
  (Variables|/Script/Engine.SpringArmComponent|SetTargetArmLength _springarm (Math|Interpolation|FInterpTo (Variables|/Script/Engine.SpringArmComponent|GetTargetArmLength _springarm) _output_get (Utilities|Time|GetWorldDeltaSeconds) 25.0)))